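; BP_SacrificialTree is a puzzle actor that consumes tagged BP_Puzzle2Object sacrifices and rewards completion with a helper NPC.
; Its sphere overlap plays an audio cue for the maze character and destroys and counts matching objects.
; At the target count it spawns BP_HelperNPC, passes it fetch and carry targets, starts GetObject, then destroys itself.
; StartFade and EndFade drive a timeline over the model's dynamic material opacity.
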(event OnComponentBeginOverlap(Sphere)
  (params (OverlappedComponent :type Primitive%20Component%20Object%20Reference) (OtherActor :type Actor%20Object%20Reference) (OtherComp :type Primitive%20Component%20Object%20Reference) (OtherBodyIndex :type Integer) (bFromSweep :type Boolean) (SweepResult :type Hit%20Result%20Structure%20%28by%20ref%29))
  (bind _audiocue (Variables|Default|GetAudioCue))
  ;[0.8941 0.3481 0.5488 0.5] Collect Sacrifical Object
  (Utilities|Casting|CastToBP_MazeCharacter OtherActor
    (:then
      (Utilities|IsValid _audiocue
        (:Is%20Valid
          (Audio|PlaySoundatLocation _audiocue (Transformation|GetActorLocation) "0, 0, 0" 1.0 1.0 0.0 0 0 0 0))
        (:Is%20Not%20Valid
          _)))
    (:CastFailed
      _))
  (bind _asbp_puzzle_2object (Utilities|Casting|CastToBP_Puzzle2Object OtherActor))
  (if (Actor|ActorHasTag _asbp_puzzle_2object (Variables|Default|GetObjectType))
    (Actor|DestroyActor _asbp_puzzle_2object)
    (bind _result (Math|Integer|IncrementInt (Variables|Default|GetNumObject))
      (:%20%20
        (bind _output_get (Variables|Default|SetNumObject _result))
        ;[0.7605 0.5271 1 0.5] Spawn NPC
        (if (== _output_get (Variables|Default|GetTotalObject))
          (bind _output_get_2 (Variables|Default|SetSpawn%20Transform (Variables|Default|GetSpawn%20Transform)))
          (bind _returnvalue (AI|SpawnAIFromClass "/Game/Blueprints/Characters/BP_HelperNPC.BP_HelperNPC_C" 0 (.location _output_get_2) "0, 0, 0" false 0))
          (bind _asbp_helper_npc (Utilities|Casting|CastToBP_HelperNPC _returnvalue))
          (Variables|/Game/Blueprints/Characters/BP_HelperNPC.BP_HelperNPC_C|SetObjectToGet _asbp_helper_npc (Variables|Default|GetObject%20to%20Get))
          (Variables|/Game/Blueprints/Characters/BP_HelperNPC.BP_HelperNPC_C|SetCarryTo _asbp_helper_npc (Variables|Default|GetCarry%20To))
          (Default|GetObject _asbp_helper_npc)
          (Actor|DestroyActor))))))

(event EventEndFade
  ;[0.7605 0.5271 1 0.5] Fade In/Out
  (bind _fadeamount (Timeline|FadeTimeline Reverse)
    (:Update
      (Rendering|Material|SetScalarParameterValue (Variables|Default|GetDynamicMaterial) "Opacity" (- 1.0 (* _fadeamount (- 1.0 (Variables|Default|GetEndingFadeAmount)))) :!class /Script/Engine.MaterialInstanceDynamic))))

(event EventStartFade
  ;[0.7605 0.5271 1 0.5] Fade In/Out
  (bind _fadeamount (Timeline|FadeTimeline Play)
    (:Update
      (Rendering|Material|SetScalarParameterValue (Variables|Default|GetDynamicMaterial) "Opacity" (- 1.0 (* _fadeamount (- 1.0 (Variables|Default|GetEndingFadeAmount)))) :!class /Script/Engine.MaterialInstanceDynamic))))

(fn ConstructionScript
  (Variables|Default|SetAudioCue (Variables|Default|GetAudioCue))
  (bind _returnvalue (Rendering|Material|CreateDynamicMaterialInstance (Variables|Default|GetModel) 0 (Variables|Default|GetFadeMaterial) "None" :!class /Script/Engine.PrimitiveComponent))
  (bind _output_get (Variables|Default|SetDynamicMaterial _returnvalue))
  (Rendering|Material|SetMaterial (Variables|Default|GetModel) 0 _output_get))