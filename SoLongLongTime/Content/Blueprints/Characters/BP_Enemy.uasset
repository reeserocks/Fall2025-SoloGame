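; BP_Enemy is an AI enemy that roams randomly over the navmesh, playing a monster sound at each destination.
; When PawnSensing sees the player, it chases with AI MoveTo, and a retriggerable delay resumes roaming after sightings stop.
; On reaching the player it plays an attack montage and sound, subtracts random damage from PlayerHealth and shows the game over widget at zero, using CanAttack as a brief cooldown.
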(event OnSeePawn(PawnSensing)
  (params (Pawn :type Pawn%20Object%20Reference))
  ;[0.3287 0.6258 1 0.5] Move Based on On See Pawn
  (Utilities|FlowControl|Sequence
    (:then_0
      (CallFunction|FollowPlayer Pawn))
    (:then_1
      (Utilities|FlowControl|RetriggerableDelay 2.0)
      (CallFunction|RandomRoam))))

(event Custom|FollowPlayer
  (params (Pawn :type Pawn%20Object%20Reference))
  ;[0.8941 0.3481 0.5488 0.5] Follow Player
  (bind _asbp_third_person_character (Utilities|Casting|CastToBP_ThirdPersonCharacter Pawn))
  (AI|AIMoveTo self "0, 0, 0" _asbp_third_person_character 25.0 false
    (:OnSuccess
      ;[0.7605 0.5271 1 0.5] Attack Player and Apply Damage
      (if (Variables|Default|GetcanAttack?)
        (Variables|Default|SetcanAttack? false)
        (Animation|PlayAnimMontage "/Game/Animations/Enemy/AM_enemy_attack.AM_enemy_attack" 1.0 "None")
        (Audio|PlaySound2D "/Game/Sounds/attack.attack" 1.0 1.0 0.0 0 0)
        (bind _returnvalue (Game|Damage|ApplyDamage _asbp_third_person_character (Math|Random|RandomFloatinRange 8.0 12.0) 0 0))
        (bind _output_get (Variables|/Game/ThirdPerson/Blueprints/BP_ThirdPersonCharacter.BP_ThirdPersonCharacter_C|SetPlayerHealth _asbp_third_person_character (- (Variables|/Game/ThirdPerson/Blueprints/BP_ThirdPersonCharacter.BP_ThirdPersonCharacter_C|GetPlayerHealth _asbp_third_person_character) _returnvalue)))
        (if (<= _output_get 0.0)
          (bind _returnvalue_2 (UserInterface|CreateWidget "/Game/Blueprints/Widgets/WBP_GameOver.WBP_GameOver_C"))
          (UserInterface|Viewport|AddtoViewport _returnvalue_2 0)
          (else
            (Utilities|FlowControl|Delay 0.2)
            (Variables|Default|SetcanAttack? true)))))))

(event Custom|RandomRoam
  ;[0.7605 0.5271 1 0.5] Random Roam
  (AI|AIMoveTo self (.RandomLocation (AI|Navigation|GetRandomReachablePointinRadius (Transformation|GetActorLocation) 5e+03 0 0)) 0 5.0 false
    (:OnSuccess
      (Audio|PlaySoundatLocation "/Game/Sounds/monster.monster" (Transformation|GetActorLocation) "0, 0, 0" 0.5 1.0 0.0 "/Game/Sounds/SoundAttenuation.SoundAttenuation" 0 0 0)
      (CallFunction|RandomRoam))))

(event EventBeginPlay
  ;[0.3287 0.6258 1 0.5] Call Random Roam First
  (CallFunction|RandomRoam))

(fn ConstructionScript)