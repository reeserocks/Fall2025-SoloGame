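; Idle NPC that acts as a checkpoint and supply point for the third-person player character.
; When the player enters its sphere collider, it shows a dialogue text, restores a random amount of health, tops up ammo within a cap and sets the player's respawn transform to its RespawnPoint.
; When the player leaves, it hides the text and picks a new random line from DialogueOptions for the next visit.
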(event OnComponentEndOverlap(SphereCollider)
  (params (OverlappedComponent :type Primitive%20Component%20Object%20Reference) (OtherActor :type Actor%20Object%20Reference) (OtherComp :type Primitive%20Component%20Object%20Reference) (OtherBodyIndex :type Integer))
  ;[1 0.5271 0.6724] set dialogue
  (Utilities|Casting|CastToBP_ThirdPersonCharacter OtherActor)
  (CallFunction|PickDialogue)
  (Rendering|SetVisibility (Variables|Default|GetTextRender) false false))

(event OnComponentBeginOverlap(SphereCollider)
  (params (OverlappedComponent :type Primitive%20Component%20Object%20Reference) (OtherActor :type Actor%20Object%20Reference) (OtherComp :type Primitive%20Component%20Object%20Reference) (OtherBodyIndex :type Integer) (bFromSweep :type Boolean) (SweepResult :type Hit%20Result%20Structure%20%28by%20ref%29))
  ;[1 0.5271 0.6724] set dialogue
  (bind _asbp_third_person_character (Utilities|Casting|CastToBP_ThirdPersonCharacter OtherActor))
  (Rendering|SetVisibility (Variables|Default|GetTextRender) true false)
  (CallFunction|HealPlayer _asbp_third_person_character)
  (CallFunction|AddAmmo _asbp_third_person_character)
  (Variables|/Game/ThirdPerson/Blueprints/BP_ThirdPersonCharacter.BP_ThirdPersonCharacter_C|SetRespawnPos _asbp_third_person_character (Transformation|GetWorldTransform (Variables|Default|GetRespawnPoint))))

(event Custom|HealPlayer
  (params (As%20BP_ThirdPersonCharacter :type BP%20Third%20Person%20Character%20Object%20Reference))
  ;[0.3287 0.6258 1 0.5] Add Health
  (if (< (Variables|/Game/ThirdPerson/Blueprints/BP_ThirdPersonCharacter.BP_ThirdPersonCharacter_C|GetPlayerHealth As%20BP_ThirdPersonCharacter) 1e+02)
    (Variables|/Game/ThirdPerson/Blueprints/BP_ThirdPersonCharacter.BP_ThirdPersonCharacter_C|SetPlayerHealth As%20BP_ThirdPersonCharacter (Math|Float|Clamp(Float) (+ (Math|Random|RandomFloatinRange 8.0 25.0) (Variables|/Game/ThirdPerson/Blueprints/BP_ThirdPersonCharacter.BP_ThirdPersonCharacter_C|GetPlayerHealth As%20BP_ThirdPersonCharacter)) 0.0 1e+02))))

(event Custom|AddAmmo
  (params (As%20BP_ThirdPersonCharacter :type BP%20Third%20Person%20Character%20Object%20Reference))
  ;[0.3287 0.6258 1 0.5] Add Ammo
  (if (< (Variables|/Game/ThirdPerson/Blueprints/BP_ThirdPersonCharacter.BP_ThirdPersonCharacter_C|GetAmmo As%20BP_ThirdPersonCharacter) 2e+01)
    (Variables|/Game/ThirdPerson/Blueprints/BP_ThirdPersonCharacter.BP_ThirdPersonCharacter_C|SetAmmo As%20BP_ThirdPersonCharacter (Math|Float|Clamp(Float) (+ (Variables|/Game/ThirdPerson/Blueprints/BP_ThirdPersonCharacter.BP_ThirdPersonCharacter_C|GetAmmo As%20BP_ThirdPersonCharacter) 5.0) 0.0 2e+01))))

(event Custom|PickDialogue
  (bind _dialogueoptions (Variables|Default|GetDialogueOptions))
  ;[0.7605 0.5271 1] return random array value
  (Utilities|Array|Shuffle _dialogueoptions)
  (Rendering|Components|TextRender|SetText (Variables|Default|GetTextRender) (Utilities|Text|ToText(String) (Utilities|Array|Get(acopy) _dialogueoptions (Math|Random|RandomIntegerinRange 0 (- (Utilities|Array|Length _dialogueoptions) 1))))))

(event EventBeginPlay
  ;[1 0.5271 0.6724] set dialogue
  (CallFunction|PickDialogue)
  (Rendering|SetVisibility (Variables|Default|GetTextRender) false false))

(fn ConstructionScript)