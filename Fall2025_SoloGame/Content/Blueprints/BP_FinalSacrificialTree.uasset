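; BP_FinalSacrificialTree is a tree prop whose mesh can fade toward a configurable opacity and back.
; The construction script assigns the configured static mesh and a dynamic instance of the fade material on its first slot.
; StartFade plays a timeline that lowers the material's Opacity parameter from fully opaque toward EndingFadeAmount, and EndFade reverses it.
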(event EventEndFade
  (bind _fadeamount (Timeline|FadeTimeline Reverse)
    (:Update
      (Rendering|Material|SetScalarParameterValue (Variables|Default|GetDyanmicMaterial) "Opacity" (- 1.0 (* _fadeamount (- 1.0 (Variables|Default|GetEndingFadeAmount)))) :!class /Script/Engine.MaterialInstanceDynamic))))

(event EventStartFade
  (bind _fadeamount (Timeline|FadeTimeline Play)
    (:Update
      (Rendering|Material|SetScalarParameterValue (Variables|Default|GetDyanmicMaterial) "Opacity" (- 1.0 (* _fadeamount (- 1.0 (Variables|Default|GetEndingFadeAmount)))) :!class /Script/Engine.MaterialInstanceDynamic))))

(fn ConstructionScript
  (Components|StaticMesh|SetStaticMesh (Variables|Default|GetModel) (Variables|Default|GetStatic%20Mesh))
  (bind _returnvalue (Rendering|Material|CreateDynamicMaterialInstance (Variables|Default|GetFadeMaterial) "None" "None" :!class /Script/Engine.KismetMaterialLibrary))
  (bind _output_get (Variables|Default|SetDyanmicMaterial _returnvalue))
  (Rendering|Material|SetMaterial (Variables|Default|GetModel) 0 _output_get))