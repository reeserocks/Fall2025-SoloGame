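; Projectile actor that damages enemies on impact.
; On hit it disables sphere collision, fires a radial force impulse and spawns a Niagara burst aligned to the surface normal.
; Actors tagged Enemy take random damage, which is subtracted directly from BP_Enemy's health variable and printed while the enemy survives.
; At zero health the enemy's mesh switches to physics simulation, then enemy and projectile are destroyed after a short delay.
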(event Collision|EventHit
  (params (MyComp :type Primitive%20Component%20Object%20Reference) (Other :type Actor%20Object%20Reference) (OtherComp :type Primitive%20Component%20Object%20Reference) (bSelfMoved :type Boolean) (HitLocation :type Vector :default "0, 0, 0") (HitNormal :type Vector :default "0, 0, 0") (NormalImpulse :type Vector :default "0, 0, 0") (Hit :type Hit%20Result%20Structure%20%28by%20ref%29))
  (bind (_bblockinghit _binitialoverlap _time _distance _location _impactpoint _normal) (Collision|BreakHitResult Hit))
  (Collision|SetCollisionEnabled (Variables|Default|GetSphere) "NoCollision")
  (Class|RadialForceComponent|FireImpulse (Variables|Default|GetRadialForce))
  (Niagara|SpawnSystematLocation "/Game/Pack_Simple_Particle_Burst/01_Niagara_Systems/NS_Simple_Burst_Level_1.NS_Simple_Burst_Level_1" _location (Math|Rotator|MakeRotfromX _normal) "1.000000,1.000000,1.000000" false)
  (Utilities|IsValid Other
    (:Is%20Valid
      (if (Actor|ActorHasTag Other "Enemy")
        (bind _returnvalue (Game|Damage|ApplyDamage Other (Math|Random|RandomFloatinRange 1e+01 15.0) 0 0))
        (bind _asbp_enemy (Utilities|Casting|CastToBP_Enemy Other))
        (bind _output_get (Variables|/Game/Blueprints/Characters/BP_Enemy.BP_Enemy_C|SetenemyHealth _asbp_enemy (- (Variables|/Game/Blueprints/Characters/BP_Enemy.BP_Enemy_C|GetenemyHealth _asbp_enemy) _returnvalue)))
        (if (<= _output_get 0.0)
          (Physics|SetSimulatePhysics (Variables|/Script/Engine.Character|GetMesh _asbp_enemy) true)
          (Utilities|FlowControl|Delay 1.5)
          (Actor|DestroyActor _asbp_enemy)
          (Actor|DestroyActor)
          (else
            (Development|PrintString (Utilities|String|Append "Enemy Health " (Utilities|String|ToString(Float) _output_get)))
            (Actor|DestroyActor)))
        (else
          (Actor|DestroyActor))))))

(fn ConstructionScript)