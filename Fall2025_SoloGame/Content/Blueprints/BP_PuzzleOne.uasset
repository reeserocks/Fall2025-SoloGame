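; BP_PuzzleOne is a puzzle trigger actor that counts grabbable ingredient objects placed into it.
; When a BP_GrabObject begins overlapping, it increments a counter, disables that object's model collision and prints the current count.
; Reaching three ingredients prints a completion message, with no further effect beyond the debug text.
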(event Custom|AddValue
  (bind _result (Math|Integer|IncrementInt (Variables|Default|GetNumIngredient))
    (:%20%20
      (bind _output_get (Variables|Default|SetNumIngredient _result))
      (if (== _output_get 3)
        (Development|PrintString "Puzzle 1 Complete!")))))

(event Collision|EventActorBeginOverlap
  (params (OtherActor :type Actor%20Object%20Reference))
  (bind _asbp_grab_object (Utilities|Casting|CastToBP_GrabObject OtherActor))
  (if (<= (Variables|Default|GetNumIngredient) 3)
    (CallFunction|AddValue)
    (Collision|SetCollisionEnabled (Variables|/Game/Blueprints/BP_GrabObject.BP_GrabObject_C|GetModel _asbp_grab_object) "NoCollision")
    (Development|PrintString (Utilities|String|ToString(Integer) (Variables|Default|GetNumIngredient)))))

(fn ConstructionScript)