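; BP_MemoryBad is a hazard actor that slows and damages the third-person character inside its Sphere.
; Overlap events cache the character, toggle an overlap flag and lower or restore walk speed.
; While overlapping, Tick feeds a one-second Delay into the Damage event, so a pending hit still lands after exit.
; Damage calls ApplyDamage, subtracts the returned amount directly from PlayerHealth and prints the result.
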(event OnComponentBeginOverlap(Sphere)
  (params (OverlappedComponent :type Primitive%20Component%20Object%20Reference) (OtherActor :type Actor%20Object%20Reference) (OtherComp :type Primitive%20Component%20Object%20Reference) (OtherBodyIndex :type Integer) (bFromSweep :type Boolean) (SweepResult :type Hit%20Result%20Structure%20%28by%20ref%29))
  (bind _asbp_third_person_character (Utilities|Casting|CastToBP_ThirdPersonCharacter OtherActor))
  (bind _output_get (Variables|Default|SetAs%20BP%20Third%20Person%20Character _asbp_third_person_character))
  (Variables|Default|SetisOverlapping? true)
  (Variables|/Script/Engine.CharacterMovementComponent|SetMaxWalkSpeed (Variables|/Script/Engine.Character|GetCharacterMovement _output_get) 2e+02))

(event OnComponentEndOverlap(Sphere)
  (params (OverlappedComponent :type Primitive%20Component%20Object%20Reference) (OtherActor :type Actor%20Object%20Reference) (OtherComp :type Primitive%20Component%20Object%20Reference) (OtherBodyIndex :type Integer))
  (Utilities|Casting|CastToBP_ThirdPersonCharacter OtherActor)
  (Variables|Default|SetisOverlapping? false)
  (Variables|/Script/Engine.CharacterMovementComponent|SetMaxWalkSpeed (Variables|/Script/Engine.Character|GetCharacterMovement (stale OnComponentBeginOverlap(Sphere) _output_get)) 6e+02))

(event Custom|Damage
  (bind _as_bp_third_person_character (Variables|Default|GetAs%20BP%20Third%20Person%20Character))
  ;[0.8941 0.3481 0.5488 0.5] Damage Loop
  (bind _returnvalue (Game|Damage|ApplyDamage _as_bp_third_person_character 2.0 0 0))
  (bind _output_get (Variables|/Game/ThirdPerson/Blueprints/BP_ThirdPersonCharacter.BP_ThirdPersonCharacter_C|SetPlayerHealth _as_bp_third_person_character (- (Variables|/Game/ThirdPerson/Blueprints/BP_ThirdPersonCharacter.BP_ThirdPersonCharacter_C|GetPlayerHealth _as_bp_third_person_character) _returnvalue)))
  (Development|PrintString (Utilities|String|ToString(Float) _output_get)))

(event EventTick
  (params (DeltaSeconds :type Float%20%28single-precision%29))
  (if (Variables|Default|GetisOverlapping?)
    (Utilities|FlowControl|Delay 1.0)
    (CallFunction|Damage)))

(fn ConstructionScript)