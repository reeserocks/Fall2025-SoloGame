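; BP_Puzzle2Object is a maze puzzle actor whose mesh, material, tags and sound come from variables.
; On BeginPlay it applies the static mesh and material to its Model component and sets its actor Tags from ObjectType.
; When BP_MazeCharacter overlaps it, a 2D sound plays, gated by a SoundPlayed flag that resets when the character's overlap ends.
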(event Collision|EventActorBeginOverlap
  (params (OtherActor :type Actor%20Object%20Reference))
  ;[0.7605 0.5271 1 0.5] Play Sound on Overlap
  (Utilities|Casting|CastToBP_MazeCharacter OtherActor)
  (if (not (Variables|Default|GetsoundPlayed?))
    (Audio|PlaySound2D (Variables|Default|GetSound) 1.0 1.0 0.0 0 0)
    (Variables|Default|SetsoundPlayed? true)))

(event Collision|EventActorEndOverlap
  (params (OtherActor :type Actor%20Object%20Reference))
  ;[0.7605 0.5271 1 0.5] Play Sound on Overlap
  (Utilities|Casting|CastToBP_MazeCharacter OtherActor)
  (Variables|Default|SetsoundPlayed? false))

(event EventBeginPlay
  ;[0.3287 0.6258 1 0.5] Set Instance Static Mesh
  (Components|StaticMesh|SetStaticMesh (Variables|Default|GetModel) (Variables|Default|GetStaticMesh))
  (Rendering|Material|SetMaterial (Variables|Default|GetModel) 0 (Variables|Default|GetMaterial))
  (Variables|Default|SetTags (Variables|Default|GetObjectType)))

(fn ConstructionScript)