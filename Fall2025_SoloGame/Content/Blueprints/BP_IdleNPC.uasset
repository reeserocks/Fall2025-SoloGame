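; Idle NPC that shows random dialogue text and resupplies the third-person player when they step into its sphere trigger.
; On overlap it reveals the text and tops up the player's health by a random amount and ammo by a fixed amount, both clamped to a maximum.
; When the player leaves, it picks a new random line from the shuffled dialogue array and hides the text.
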(event OnComponentEndOverlap(SphereCollider)
  (params (OverlappedComponent :type Primitive%20Component%20Object%20Reference) (OtherActor :type Actor%20Object%20Reference) (OtherComp :type Primitive%20Component%20Object%20Reference) (OtherBodyIndex :type Integer))
  ;[1 0.5271 0.6724] set dialogue
  (Utilities|Casting|CastToBP_ThirdPersonCharacter OtherActor)
  (CallFunction|PickDialogue)
  (Rendering|SetVisibility (Variables|Default|GetTextRender) false false))

(event OnComponentBeginOverlap(SphereCollider)
  (params (OverlappedComponent :type Primitive%20Component%20Object%20Reference) (OtherActor :type Actor%20Object%20Reference) (OtherComp :type Primitive%20Component%20Object%20Reference) (OtherBodyIndex :type Integer) (bFromSweep :type Boolean) (SweepResult :type Hit%20Result%20Structure%20%28by%20ref%29))
  ;[1 0.5271 0.6724] set dialogue
  (bind _asbp_third_person_character (Utilities|Casting|CastToBP_ThirdPersonCharacter OtherActor))
  (Rendering|SetVisibility (Variables|Default|GetTextRender) true false)
  (CallFunction|HealPlayer _asbp_third_person_character)
  (CallFunction|AddAmmo _asbp_third_person_character))

(event Custom|HealPlayer
  (params (As%20BP_ThirdPersonCharacter :type BP%20Third%20Person%20Character%20Object%20Reference))
  ;[0.3287 0.6258 1 0.5] Add Health
  (if (< (Variables|/Game/ThirdPerson/Blueprints/BP_ThirdPersonCharacter.BP_ThirdPersonCharacter_C|GetPlayerHealth As%20BP_ThirdPersonCharacter) 1e+02)
    (bind _output_get (Variables|/Game/ThirdPerson/Blueprints/BP_ThirdPersonCharacter.BP_ThirdPersonCharacter_C|SetPlayerHealth As%20BP_ThirdPersonCharacter (Math|Float|Clamp(Float) (+ (Math|Random|RandomFloatinRange 8.0 25.0) (Variables|/Game/ThirdPerson/Blueprints/BP_ThirdPersonCharacter.BP_ThirdPersonCharacter_C|GetPlayerHealth As%20BP_ThirdPersonCharacter)) 0.0 1e+02)))
    (Development|PrintString (Utilities|String|Append "Player Gains Health: " (Utilities|String|ToString(Float) _output_get)))))

(event Custom|AddAmmo
  (params (As%20BP_ThirdPersonCharacter :type BP%20Third%20Person%20Character%20Object%20Reference))
  ;[0.3287 0.6258 1 0.5] Add Ammo
  (if (< (Variables|/Game/ThirdPerson/Blueprints/BP_ThirdPersonCharacter.BP_ThirdPersonCharacter_C|GetAmmo As%20BP_ThirdPersonCharacter) 20)
    (bind _output_get (Variables|/Game/ThirdPerson/Blueprints/BP_ThirdPersonCharacter.BP_ThirdPersonCharacter_C|SetAmmo As%20BP_ThirdPersonCharacter (Math|Integer|Clamp(Integer) (+ (Variables|/Game/ThirdPerson/Blueprints/BP_ThirdPersonCharacter.BP_ThirdPersonCharacter_C|GetAmmo As%20BP_ThirdPersonCharacter) 5) 0 20)))
    (Development|PrintString (Utilities|String|Append "Player Gains Ammo: " (Utilities|String|ToString(Integer) _output_get)))))

(event Custom|PickDialogue
  (bind _dialogueoptions (Variables|Default|GetDialogueOptions))
  ;[0.7605 0.5271 1] return random array value
  (Utilities|Array|Shuffle _dialogueoptions)
  (Rendering|Components|TextRender|SetText (Variables|Default|GetTextRender) (Utilities|Text|ToText(String) (Utilities|Array|Get(acopy) _dialogueoptions (Math|Random|RandomIntegerinRange 0 (- (Utilities|Array|Length _dialogueoptions) 1))))))

(event EventBeginPlay
  ;[1 0.5271 0.6724] set dialogue
  (CallFunction|PickDialogue))

(fn ConstructionScript)