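; BP_EnemySpawner is an area spawner that scales enemy reinforcements to player health, sending fewer as health drops.
; Box overlaps track whether the player is inside.
; While inside, Tick runs a health check whenever exactly one enemy overlaps the spawner, so an empty area triggers nothing.
; The check spawns one to three BP_Enemy AI at random navigable points around the player and starts each roaming.
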(event OnComponentBeginOverlap(Box)
  (params (OverlappedComponent :type Primitive%20Component%20Object%20Reference) (OtherActor :type Actor%20Object%20Reference) (OtherComp :type Primitive%20Component%20Object%20Reference) (OtherBodyIndex :type Integer) (bFromSweep :type Boolean) (SweepResult :type Hit%20Result%20Structure%20%28by%20ref%29))
  ;[0.3287 0.6258 1 0.5] Check if Overlapping
  (if (Actor|ActorHasTag OtherActor "Player")
    (bind _asbp_third_person_character (Utilities|Casting|CastToBP_ThirdPersonCharacter OtherActor))
    (Variables|Default|SetisOverlapping? true)))

(event OnComponentEndOverlap(Box)
  (params (OverlappedComponent :type Primitive%20Component%20Object%20Reference) (OtherActor :type Actor%20Object%20Reference) (OtherComp :type Primitive%20Component%20Object%20Reference) (OtherBodyIndex :type Integer))
  ;[0.3287 0.6258 1 0.5] Check if Overlapping
  (if (Actor|ActorHasTag OtherActor "Player")
    (Utilities|Casting|CastToBP_ThirdPersonCharacter OtherActor)
    (Variables|Default|SetisOverlapping? false)))

(event Custom|SpawnEnemy
  ;[0.8941 0.3481 0.5488 0.5] Spawn Enemy
  (bind _randomlocation (Class|NavigationSystemV1|GetRandomLocationinNavigableRadius (Transformation|GetActorLocation (Game|GetPlayerCharacter 0)) 5e+03 0 0))
  (bind _returnvalue (AI|SpawnAIFromClass "/Game/Blueprints/BP_Enemy.BP_Enemy_C" 0 _randomlocation "0, 0, 0" false 0))
  (bind _asbp_enemy (Utilities|Casting|CastToBP_Enemy _returnvalue))
  (Default|RandomRoam _asbp_enemy))

(event Custom|HealthCheck
  (params (Other%20Actor :type Actor%20Object%20Reference))
  ;[0.7605 0.5271 1 0.5] Spawn Enemies Based on Player Health
  (bind _asbp_third_person_character (Utilities|Casting|CastToBP_ThirdPersonCharacter Other%20Actor))
  (if (<= (Variables|/Game/ThirdPerson/Blueprints/BP_ThirdPersonCharacter.BP_ThirdPersonCharacter_C|GetPlayerHealth _asbp_third_person_character) 7e+01)
    (if (<= (Variables|/Game/ThirdPerson/Blueprints/BP_ThirdPersonCharacter.BP_ThirdPersonCharacter_C|GetPlayerHealth _asbp_third_person_character) 3e+01)
      (CallFunction|SpawnEnemy)
      (else
        (CallFunction|SpawnEnemy)
        (CallFunction|SpawnEnemy)))
    (else
      (CallFunction|SpawnEnemy)
      (CallFunction|SpawnEnemy)
      (CallFunction|SpawnEnemy))))

(event EventTick
  (params (DeltaSeconds :type Float%20%28single-precision%29))
  (bind _overlappingactors (Collision|GetOverlappingActors "/Game/Blueprints/BP_Enemy.BP_Enemy_C" :!class /Script/Engine.Actor))
  ;[0.3287 0.6258 1 0.5] Spawn More Enemies While Player in Range
  (if (Variables|Default|GetisOverlapping?)
    (if (and (<= (Utilities|Array|Length _overlappingactors) 1) (Utilities|Array|IsValidIndex _overlappingactors))
      (CallFunction|HealthCheck (stale OnComponentBeginOverlap(Box) _asbp_third_person_character)))))

(fn ConstructionScript)