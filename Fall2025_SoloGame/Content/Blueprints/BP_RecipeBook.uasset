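; BP_RecipeBook is an interactable recipe book that opens a recipe book widget when the player presses interact nearby.
; Its Collider overlap with BP_ThirdPersonCharacter enables the actor's input and shows a "Press E" prompt; leaving disables input and removes the prompt.
; IA_Interact removes the prompt and adds WBP_RecipeBook to the viewport, using the widget's BookOnScreen flag to avoid duplicates.
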(event OnComponentBeginOverlap(Collider)
  (params (OverlappedComponent :type Primitive%20Component%20Object%20Reference) (OtherActor :type Actor%20Object%20Reference) (OtherComp :type Primitive%20Component%20Object%20Reference) (OtherBodyIndex :type Integer) (bFromSweep :type Boolean) (SweepResult :type Hit%20Result%20Structure%20%28by%20ref%29))
  (Utilities|Casting|CastToBP_ThirdPersonCharacter OtherActor)
  (Input|EnableInput (Game|GetPlayerController 0))
  (if (not (Variables|Default|GetisOnScreen?))
    (bind _returnvalue (UserInterface|CreateWidget "/Game/Blueprints/Widgets/WBP_Interact.WBP_Interact_C" (Game|GetPlayerController 0)))
    (Rendering|Components|TextRender|SetText (Variables|/Game/Blueprints/Widgets/WBP_Interact.WBP_Interact_C|GetInteractText _returnvalue) "Press E to look at recipe.")
    (UserInterface|Viewport|AddtoViewport _returnvalue 0)
    (Variables|Default|SetisOnScreen? true)))

(event OnComponentEndOverlap(Collider)
  (params (OverlappedComponent :type Primitive%20Component%20Object%20Reference) (OtherActor :type Actor%20Object%20Reference) (OtherComp :type Primitive%20Component%20Object%20Reference) (OtherBodyIndex :type Integer))
  (Utilities|Casting|CastToBP_ThirdPersonCharacter OtherActor)
  (Input|DisableInput (Game|GetPlayerController 0))
  (Utilities|IsValid (stale OnComponentBeginOverlap(Collider) _returnvalue)
    (:Is%20Valid
      (Widget|RemovefromParent (stale OnComponentBeginOverlap(Collider) _returnvalue))
      (Variables|Default|SetisOnScreen? false))))

(event Input|EnhancedActionEvents|EnhancedInputActionIA_Interact
  (params (ActionValue :type Boolean) (ElapsedSeconds :type Float%20%28double-precision%29) (TriggeredSeconds :type Float%20%28double-precision%29) (InputAction :type Input%20Action%20Object%20Reference :default "/Game/Input/Actions/IA_Interact.IA_Interact"))
  (:Started
    (Utilities|IsValid (stale OnComponentBeginOverlap(Collider) _returnvalue)
      (:Is%20Valid
        (Widget|RemovefromParent (stale OnComponentBeginOverlap(Collider) _returnvalue))
        (if (not (Variables|/Game/Blueprints/Widgets/WBP_RecipeBook.WBP_RecipeBook_C|GetbookOnScreen? (stale _returnvalue)))
          (bind _returnvalue (UserInterface|CreateWidget "/Game/Blueprints/Widgets/WBP_RecipeBook.WBP_RecipeBook_C" (Game|GetPlayerController 0)))
          (UserInterface|Viewport|AddtoViewport _returnvalue 0)
          (Variables|/Game/Blueprints/Widgets/WBP_RecipeBook.WBP_RecipeBook_C|SetbookOnScreen? _returnvalue true))))))

(fn ConstructionScript)