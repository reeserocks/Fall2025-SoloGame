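; BP_MemoryGood is a "good memory" actor that shows a text widget, plays a sound and heals the player nearby.
; Sphere overlap by BP_ThirdPersonCharacter adds WBP_Memory with the instance's text; leaving removes it.
; While overlapping below full health, Tick feeds a Delay that throttles Heal to small, clamped increments about once per second.
; The construction script applies the configurable mesh to the Cube.
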(event OnComponentBeginOverlap(Sphere)
  (params (OverlappedComponent :type Primitive%20Component%20Object%20Reference) (OtherActor :type Actor%20Object%20Reference) (OtherComp :type Primitive%20Component%20Object%20Reference) (OtherBodyIndex :type Integer) (bFromSweep :type Boolean) (SweepResult :type Hit%20Result%20Structure%20%28by%20ref%29))
  (bind _asbp_third_person_character (Utilities|Casting|CastToBP_ThirdPersonCharacter OtherActor))
  (Variables|Default|SetAs%20BP%20Third%20Person%20Character _asbp_third_person_character)
  (Variables|Default|SetisOverlapping? true)
  (if (not (Variables|Default|GetisOnScreen?))
    (bind _returnvalue (UserInterface|CreateWidget "/Game/Blueprints/Widgets/WBP_Memory.WBP_Memory_C" (Game|GetPlayerController 0)))
    (Rendering|Components|TextRender|SetText (Variables|/Game/Blueprints/Widgets/WBP_Memory.WBP_Memory_C|GetMemoryText _returnvalue) (Variables|Default|GetMemoryText))
    (UserInterface|Viewport|AddtoViewport _returnvalue 0)
    (Variables|Default|SetisOnScreen? true)
    (Audio|PlaySoundatLocation (Variables|Default|GetSound) (Transformation|GetActorLocation) "0, 0, 0" 1.0 1.0 0.0 "/Game/Sounds/SoundAttenuation.SoundAttenuation" 0 0 0)))

(event OnComponentEndOverlap(Sphere)
  (params (OverlappedComponent :type Primitive%20Component%20Object%20Reference) (OtherActor :type Actor%20Object%20Reference) (OtherComp :type Primitive%20Component%20Object%20Reference) (OtherBodyIndex :type Integer))
  (Utilities|Casting|CastToBP_ThirdPersonCharacter OtherActor)
  (Variables|Default|SetisOverlapping? false)
  (Widget|RemovefromParent (stale OnComponentBeginOverlap(Sphere) _returnvalue))
  (Variables|Default|SetisOnScreen? false))

(event Custom|Heal
  (bind _as_bp_third_person_character (Variables|Default|GetAs%20BP%20Third%20Person%20Character))
  ;[0.8941 0.3481 0.5488 0.5] Heal Loop
  (Variables|/Game/ThirdPerson/Blueprints/BP_ThirdPersonCharacter.BP_ThirdPersonCharacter_C|SetPlayerHealth _as_bp_third_person_character (Math|Float|Clamp(Float) (+ (Variables|/Game/ThirdPerson/Blueprints/BP_ThirdPersonCharacter.BP_ThirdPersonCharacter_C|GetPlayerHealth _as_bp_third_person_character) 2.0) 0.0 1e+02)))

(event EventTick
  (params (DeltaSeconds :type Float%20%28single-precision%29))
  (if (Variables|Default|GetisOverlapping?)
    (if (< (Variables|/Game/ThirdPerson/Blueprints/BP_ThirdPersonCharacter.BP_ThirdPersonCharacter_C|GetPlayerHealth (Variables|Default|GetAs%20BP%20Third%20Person%20Character)) 1e+02)
      (Utilities|FlowControl|Delay 1.0)
      (CallFunction|Heal))))

(fn ConstructionScript
  (Components|StaticMesh|SetStaticMesh (Variables|Components|GetCube) (Variables|Default|GetStaticMesh))
  (Variables|Default|SetMemoryText (Variables|Default|GetMemoryText))
  (Variables|Default|SetSound (Variables|Default|GetSound)))