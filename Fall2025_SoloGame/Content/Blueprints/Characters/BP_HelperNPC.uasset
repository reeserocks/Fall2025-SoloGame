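; Helper NPC that fetches an assigned object, delivers it, then follows the player through a repeating AI move loop.
; On BeginPlay it moves to ObjectToGet, sphere-traces for a physics body, and carries it by physics constraint at reduced speed.
; At CarryTo it releases the object, restores speed and starts following.
; Player overlap calls HealPlayer, which currently zeroes health below 100 because the random-heal clamp is unconnected.
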(event OnComponentBeginOverlap(SphereCollider)
  (params (OverlappedComponent :type Primitive%20Component%20Object%20Reference) (OtherActor :type Actor%20Object%20Reference) (OtherComp :type Primitive%20Component%20Object%20Reference) (OtherBodyIndex :type Integer) (bFromSweep :type Boolean) (SweepResult :type Hit%20Result%20Structure%20%28by%20ref%29))
  ;[0.8941 0.3481 0.5488 0.5] on overlap, heal player
  (bind _asbp_maze_character (Utilities|Casting|CastToBP_MazeCharacter OtherActor))
  (CallFunction|HealPlayer _asbp_maze_character))

(event Custom|HealPlayer
  (params (As%20BP_MazeCharacter :type BP%20Maze%20Character%20Object%20Reference))
  ;[0.3287 0.6258 1 0.5] Add Health
  (if (< (Variables|/Game/Blueprints/Characters/BP_MazeCharacter.BP_MazeCharacter_C|GetPlayerHealth As%20BP_MazeCharacter) 1e+02)
    (bind _output_get (Variables|/Game/Blueprints/Characters/BP_MazeCharacter.BP_MazeCharacter_C|SetPlayerHealth As%20BP_MazeCharacter 0.0))
    (Development|PrintString (Utilities|String|Append "Player Gains Health: " (Utilities|String|ToString(Float) _output_get)))))

(event Custom|FollowPlayer
  (bind _char_ref (Variables|Default|GetChar%20REF))
  (bind _returnvalue (Transformation|GetDistanceTo _char_ref))
  ;[0.7605 0.5271 1 0.5] Follow Player
  (if (>= _returnvalue 4e+02)
    (AI|AIMoveTo self "0, 0, 0" (Variables|Default|GetChar%20REF) 2e+02 false
      (:then
        _))
    (else
      (AI|AIMoveTo self (Math|Conversions|ToVector(Float) (+ _returnvalue 2e+02)) 0 5.0 false
        (:then
          _))))
  (Utilities|FlowControl|Delay 0.1)
  (CallFunction|FollowPlayer))

(event Custom|DeliverObject
  ;[0.3287 0.6258 1 0.5] Deliver Object
  (AI|AIMoveTo self (.ProjectedLocation (AI|Navigation|ProjectPointtoNavigation (Transformation|GetActorLocation (Variables|Default|GetCarryTo)) 0 0 "300.000000,300.000000,300.000000")) 0 1.4e+02 false
    (:OnSuccess
      (Variables|Default|SetisCarrying? false)
      (Utilities|IsValid (.HitComponent (Collision|BreakHitResult (stale Custom|GetObject _outhit)))
        (:Is%20Valid
          (Collision|SetCollisionEnabled (.HitComponent (Collision|BreakHitResult (stale Custom|GetObject _outhit))) "QueryAndPhysics")
          (Class|PhysicsConstraintComponent|BreakConstraint (Variables|Default|GetPhysicsConstraint))
          (Variables|/Script/Engine.CharacterMovementComponent|SetMaxWalkSpeed (Variables|Character|GetCharacterMovement) 6e+02)
          (CallFunction|FollowPlayer))))))

(event Custom|GetObject
  (bind _returnvalue (Transformation|GetActorLocation))
  ;[0.8941 0.3481 0.5488 0.5] get object and pick up
  (AI|AIMoveTo self "0, 0, 0" (Variables|Default|GetObjectToGet) 5.0 false
    (:OnSuccess
      (bind (_outhit _returnvalue_2) (Collision|SphereTraceForObjects _returnvalue _returnvalue 75.0 (Utilities|Array|MakeArray "ObjectTypeQuery4") false 0 "None"))
      (Utilities|IsValid (.HitComponent (Collision|BreakHitResult _outhit))
        (:Is%20Valid
          (if _returnvalue_2
            (Class|PhysicsConstraintComponent|SetConstrainedComponents (Variables|Default|GetPhysicsConstraint) (Variables|Character|GetMesh) "neck_01" (.HitComponent (Collision|BreakHitResult _outhit)) "None")
            (Variables|Default|SetisCarrying? true)
            (Variables|/Script/Engine.CharacterMovementComponent|SetMaxWalkSpeed (Variables|Character|GetCharacterMovement) 4e+02)
            (Collision|SetCollisionEnabled (.HitComponent (Collision|BreakHitResult _outhit)) "PhysicsOnly")
            (CallFunction|DeliverObject)))))))

(event EventBeginPlay
  ;[0.8941 0.3481 0.5488 0.5] Call Functions
  (bind _asbp_maze_character (Utilities|Casting|CastToBP_MazeCharacter (Game|GetPlayerCharacter 0)))
  (Variables|Default|SetChar%20REF _asbp_maze_character)
  (CallFunction|GetObject))

(fn ConstructionScript)