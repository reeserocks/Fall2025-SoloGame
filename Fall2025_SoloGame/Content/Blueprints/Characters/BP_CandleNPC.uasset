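; BP_CandleNPC is an NPC that shows a random line of floating dialogue when the player character comes near.
; An overlap sphere makes the TextRender visible when BP_ThirdPersonCharacter enters and hides it again when that character leaves.
; PickDialogue runs on BeginPlay and on each exit, shuffling DialogueOptions and setting a random entry as the text, so the next line is ready before the following approach.
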(event OnComponentEndOverlap(SphereCollider)
  (params (OverlappedComponent :type Primitive%20Component%20Object%20Reference) (OtherActor :type Actor%20Object%20Reference) (OtherComp :type Primitive%20Component%20Object%20Reference) (OtherBodyIndex :type Integer))
  ;[1 0.5271 0.6724] set dialogue
  (Utilities|Casting|CastToBP_ThirdPersonCharacter OtherActor)
  (CallFunction|PickDialogue)
  (Rendering|SetVisibility (Variables|Default|GetTextRender) false false))

(event OnComponentBeginOverlap(SphereCollider)
  (params (OverlappedComponent :type Primitive%20Component%20Object%20Reference) (OtherActor :type Actor%20Object%20Reference) (OtherComp :type Primitive%20Component%20Object%20Reference) (OtherBodyIndex :type Integer) (bFromSweep :type Boolean) (SweepResult :type Hit%20Result%20Structure%20%28by%20ref%29))
  ;[1 0.5271 0.6724] set dialogue
  (Utilities|Casting|CastToBP_ThirdPersonCharacter OtherActor)
  (Rendering|SetVisibility (Variables|Default|GetTextRender) true false))

(event Custom|PickDialogue
  (bind _dialogueoptions (Variables|Default|GetDialogueOptions))
  ;[0.7605 0.5271 1] return random array value
  (Utilities|Array|Shuffle _dialogueoptions)
  (Rendering|Components|TextRender|SetText (Variables|Default|GetTextRender) (Utilities|Text|ToText(String) (Utilities|Array|Get(acopy) _dialogueoptions (Math|Random|RandomIntegerinRange 0 (- (Utilities|Array|Length _dialogueoptions) 1))))))

(event EventBeginPlay
  ;[1 0.5271 0.6724] set dialogue
  (CallFunction|PickDialogue)
  (Rendering|SetVisibility (Variables|Default|GetTextRender) false false))

(fn ConstructionScript)